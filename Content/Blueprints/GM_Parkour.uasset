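; GM_Parkour is the game mode for a parkour level with a countdown timer, death screen and level restart.
; BeginPlay creates the HUD and death screen widgets, and Tick counts down the time once the player has moved, updating the HUD.
; When time runs out it kills BP_Player and shows the death screen, and RestartLevel reloads ThirdPersonMap only if the player has died.
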(event Custom|Restart%20Level
  (if (Variables|Default|GetPlayer%20Died)
    (Game|OpenLevel(byObjectReference) "/Game/ThirdPerson/Maps/ThirdPersonMap.ThirdPersonMap")))

(event EventBeginPlay
  ;[1 1 1] Create and set HUD
  (bind _returnvalue (UserInterface|CreateWidget "/Game/Blueprints/WBP_HUD.WBP_HUD_C"))
  (bind _output_get (Variables|Default|SetHUD _returnvalue))
  (UserInterface|Viewport|AddtoViewport _output_get 0)
  (Default|SetTime _output_get (Variables|Default|GetTime))
  ;[1 1 1] Create death screen
  (bind _returnvalue_2 (UserInterface|CreateWidget "/Game/Blueprints/WBP_DeathScreen.WBP_DeathScreen_C"))
  (Variables|Default|SetDeath%20Screen _returnvalue_2))

(event EventTick
  (params (DeltaSeconds :type Float%20%28single-precision%29))
  ;[1 1 1] Check if we should decrement the timer
  (if (and (Variables|Default|GetPlayer%20Moved) (not (Variables|Default|GetPlayer%20Died)))
    ;[1 1 1] Decrement the timer and check if it hit 0
    (if (> (- (Variables|Default|GetTime) DeltaSeconds) 0.0)
      ;[1 1 1] Player lives
      (Variables|Default|SetTime (- (Variables|Default|GetTime) DeltaSeconds))
      (else
        ;[1 1 1] Player died
        (Variables|Default|SetPlayer%20Died true)
        (Variables|Default|SetTime 0.0)
        (bind _asbp_player (Utilities|Casting|CastToBP_Player (Game|Player|GetPlayerPawn 0)))
        (Default|Die _asbp_player)
        (UserInterface|Viewport|AddtoViewport (Variables|Default|GetDeath%20Screen) 0)))
    ;[1 1 1] Set the timer in the HUD
    (Default|SetTime (Variables|Default|GetHUD) (Variables|Default|GetTime))))

(fn ConstructionScript)